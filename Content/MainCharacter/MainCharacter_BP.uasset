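; Player character Blueprint that targets Element_BP actors in front of the follow camera and can delete them.
; Each Tick, a camera-forward line trace stores any Element_BP hit as Target, which keeps its last value otherwise and is destroyed by DeleteTarget.
; BeginPlay limits the minimum camera pitch, and the I key sets mouse cursor visibility from UserIventoryUIStatus, which this graph never changes.
; An unconnected box trace is unused.
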(event EventBeginPlay
  (Variables|/Script/Engine.PlayerCameraManager|SetViewPitchMin (Game|GetPlayerCameraManager 0) -8e+01))

(event Collision|EventActorBeginOverlap
  (params (OtherActor :type Actor%20Object%20Reference)))

(event EventTick
  (params (DeltaSeconds :type Float%20%28single-precision%29))
  (bind _followcamera (Variables|Default|GetFollowCamera))
  (bind _returnvalue (Transformation|GetWorldLocation _followcamera))
  (bind _outhit (Collision|LineTraceByChannel _returnvalue (+ _returnvalue (* (Math|Vector|GetForwardVector (Transformation|GetWorldRotation _followcamera)) 1e+03)) "TraceTypeQuery1" false 0 "None" true "(R=0.000000,G=0.000000,B=0.000000,A=1.000000)" "(R=0.000000,G=0.000000,B=0.000000,A=1.000000)"))
  (bind _aselement_bp (Utilities|Casting|CastToElement_BP (.HitActor (Collision|BreakHitResult _outhit))))
  (Variables|Default|SetTarget _aselement_bp))

(event Input|KeyboardEvents|I
  (params (Key :type Key%20Structure :default "None"))
  (bind _returnvalue (Game|GetPlayerController 0))
  (:Pressed
    (if (Variables|Default|GetUserIventoryUIStatus)
      (Variables|/Script/Engine.PlayerController|SetbShowMouseCursor _returnvalue true)
      (else
        (Variables|/Script/Engine.PlayerController|SetbShowMouseCursor _returnvalue false)))))

(fn ConstructionScript)

(fn DeleteTarget
  (Actor|DestroyActor (Variables|Default|GetTarget)))